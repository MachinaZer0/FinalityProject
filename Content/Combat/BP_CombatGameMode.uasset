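; Combat game mode that spawns allies and enemies at spawn points and manages targeting and combat level transitions.
; BeginPlay possesses the last spawned ally as Leader, caches character lists, targets the first enemy and copies all characters into TurnOrder.
; Tick re-possesses Leader every frame, while Retarget moves the targeted flag and swaps highlight materials.
; EnterCombat opens Arena1; ExitCombat returns to Lvl_ThirdPerson when the enemy or all-character list is empty.
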(event `TargetInit`
  (bind _output (`|GetArrayItem` (`self.SpawnedEnemyCharacters`)))
  (set `self.Target` _output)
  (set `/Game/Combat/Characters/BP_ThirdPersonCharacter.IsTargeted` true _output)
  (`PrimitiveComponent.SetMaterial` (`Character.Mesh` _output) 0 "/Engine/MapTemplates/Materials/BasicAsset01.BasicAsset01")
  (`KismetSystemLibrary.PrintString` "EnemyTargeted"))

(event `self.ReceiveBeginPlay`
  (bind _returnvalue (`GameplayStatics.GetPlayerController` 0))
  (bind _leader (`self.Leader`))
  (bind _outactors (`GameplayStatics.GetAllActorsOfClass` "/Game/Combat/BP_SpawnPointAlly.BP_SpawnPointAlly_C"))
  (for _array_element _outactors
    (bind _returnvalue_2 (`|SpawnActorFromClass` (`/Game/Combat/BP_SpawnPoint.SpawnedEntity` _array_element) (`self.GetTransform` _array_element) "AdjustIfPossibleButAlwaysSpawn" "MultiplyWithRoot" null null))
    (set `self.Leader` _returnvalue_2))
  (`KismetSystemLibrary.PrintString` "All spawned")
  (`/Engine/EditorBlueprintResources/StandardMacros.IsValid` (`self.Leader`)
    (:`Is Valid`
      (`Controller.Possess` _returnvalue _leader)
      (`KismetSystemLibrary.PrintString` (`KismetSystemLibrary.GetDisplayName` (`Controller.K2_GetPawn` _returnvalue)))
      (`PlayerController.SetViewTargetWithBlend` _returnvalue _leader 0.0 "VTBlend_Linear" 0.0 false)
      (bind _outactors_2 (`GameplayStatics.GetAllActorsOfClass` "/Game/Combat/BP_SpawnPointEnemy.BP_SpawnPointEnemy_C"))
      (for _array_element_2 _outactors_2
        (`|SpawnActorFromClass` (`/Game/Combat/BP_SpawnPoint.SpawnedEntity` _array_element_2) (`self.GetTransform` _array_element_2) "AdjustIfPossibleButAlwaysSpawn" "MultiplyWithRoot" null null))
      (bind _outactors_3 (`GameplayStatics.GetAllActorsOfClass` "/Game/Combat/Characters/BP_ThirdPersonCharacter.BP_ThirdPersonCharacter_C"))
      (set `self.SpawnedAllCharacters` _outactors_3)
      (bind _outactors_4 (`GameplayStatics.GetAllActorsOfClass` "/Game/Combat/Characters/BP_PlayerCharacters.BP_PlayerCharacters_C"))
      (set `self.SpawnedPlayerCharacters` _outactors_4)
      (bind _outactors_5 (`GameplayStatics.GetAllActorsOfClass` "/Game/Combat/Characters/BP_EnemyCharacters.BP_EnemyCharacters_C"))
      (set `self.SpawnedEnemyCharacters` _outactors_5)
      (`self.TargetInit`)
      (set `self.TurnOrder` (`self.SpawnedAllCharacters`)))
    (:`Is Not Valid`
      (`KismetSystemLibrary.PrintString` "Possess Error"))))

(event `self.ReceiveTick`
  (params (DeltaSeconds :type "Float (single-precision)"))
  (`Controller.Possess` (`GameplayStatics.GetPlayerController` 0) (`self.Leader`)))

(fn `EnterCombat`
  (`KismetSystemLibrary.PrintString` "Entered Combat")
  (`GameplayStatics.OpenLevel` "Arena1"))

(fn `ExitCombat`
  (if (<= (`KismetArrayLibrary.Array_Length` (`self.SpawnedEnemyCharacters`)) 0)
    (`KismetSystemLibrary.PrintString` "Victory")
    (`GameplayStatics.OpenLevel` "Lvl_ThirdPerson" :!label _label)
    (elif (<= (`KismetArrayLibrary.Array_Length` (`self.SpawnedAllCharacters`)) 0)
      (`KismetSystemLibrary.PrintString` "Defeat")
      (goto _label)
      (else
        (`KismetSystemLibrary.PrintString` "Combat Persists")))))

(fn `Retarget`
  (params (NewTarget :type "/Game/Combat/Characters/BP_ThirdPersonCharacter Object Reference") (OldTarget :type "/Game/Combat/Characters/BP_ThirdPersonCharacter Object Reference"))
  (set `self.Target` NewTarget)
  (set `/Game/Combat/Characters/BP_ThirdPersonCharacter.IsTargeted` true NewTarget)
  (`PrimitiveComponent.SetMaterial` (`Character.Mesh` NewTarget) 0 "/Engine/MapTemplates/Materials/BasicAsset01.BasicAsset01")
  (set `/Game/Combat/Characters/BP_ThirdPersonCharacter.IsTargeted` false OldTarget)
  (`PrimitiveComponent.SetMaterial` (`Character.Mesh` OldTarget) 0 "/Engine/EditorMaterials/PhAT_ElemSelectedOverlappingMaterial.PhAT_ElemSelectedOverlappingMaterial")
  (`KismetSystemLibrary.PrintString` (`KismetStringLibrary.Concat_StrStr` "Now Targeting:" (`KismetSystemLibrary.GetDisplayName` NewTarget))))

(fn `UserConstructionScript`)