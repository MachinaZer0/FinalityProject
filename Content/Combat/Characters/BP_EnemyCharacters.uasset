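; Enemy character Blueprint for the combat game, handling enemy bookkeeping on death.
; Its Death event removes itself from the combat game mode's SpawnedEnemyCharacters array and prints the remaining count.
; It then destroys the actor held in the game mode's Target variable, rather than explicitly destroying itself.
; A failed first game mode cast prints an error, and construction only calls the parent script.
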(event `self.Death`
  (bind _asbp_combat_game_mode (cast `/Game/Combat/BP_CombatGameMode` (`GameplayStatics.GetGameMode`))
    (:`then`
      (bind _spawnedenemycharacters (`/Game/Combat/BP_CombatGameMode.SpawnedEnemyCharacters` _asbp_combat_game_mode))
      (`KismetArrayLibrary.Array_RemoveItem` _spawnedenemycharacters self)
      (`KismetSystemLibrary.PrintString` (`KismetStringLibrary.Concat_StrStr` "Enemies Remaining: " (`KismetStringLibrary.Conv_IntToString` (`KismetArrayLibrary.Array_Length` _spawnedenemycharacters))))
      (bind _asbp_combat_game_mode_2 (cast `/Game/Combat/BP_CombatGameMode` (`GameplayStatics.GetGameMode`)))
      (`self.K2_DestroyActor` (`/Game/Combat/BP_CombatGameMode.Target` _asbp_combat_game_mode_2)))
    (:`CastFailed`
      (`KismetSystemLibrary.PrintString` "cast failed"))))

(fn `UserConstructionScript`
  (`parent.UserConstructionScript`))