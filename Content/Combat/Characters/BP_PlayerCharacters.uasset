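; Base or shared Blueprint for player characters in combat, handling what happens when one dies.
; Death removes the character from the combat game mode's player and all-character lists, marks the Leader dead, prints the remaining player count, and calls ExitCombat without checking that count.
; Finality is an empty function, and a disconnected fragment that would zero CurrentHP and call Death never runs.
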(event `self.Death`
  (bind _asbp_combat_game_mode (cast `/Game/Combat/BP_CombatGameMode` (`GameplayStatics.GetGameMode`))
    (:`then`
      (`KismetArrayLibrary.Array_RemoveItem` (`/Game/Combat/BP_CombatGameMode.SpawnedPlayerCharacters` _asbp_combat_game_mode) self)
      (`KismetArrayLibrary.Array_RemoveItem` (`/Game/Combat/BP_CombatGameMode.SpawnedAllCharacters` _asbp_combat_game_mode) self)
      (bind _asbp_combat_game_mode_2 (cast `/Game/Combat/BP_CombatGameMode` (`GameplayStatics.GetGameMode`)))
      (set `/Game/Combat/Characters/BP_ThirdPersonCharacter.IsDead` true (`/Game/Combat/BP_CombatGameMode.Leader` _asbp_combat_game_mode_2))
      (`KismetSystemLibrary.PrintString` (`KismetStringLibrary.Conv_IntToString` (`KismetArrayLibrary.Array_Length` (`/Game/Combat/BP_CombatGameMode.SpawnedPlayerCharacters` _asbp_combat_game_mode_2))))
      (`/Game/Combat/BP_CombatGameMode.ExitCombat` _asbp_combat_game_mode_2))
    (:`CastFailed`
      (`KismetSystemLibrary.PrintString` "cast failed"))))

(fn `Finality`
  (params (EnemyTarget :type "/Game/Combat/Characters/BP_ThirdPersonCharacter Object Reference")))

(fn `UserConstructionScript`
  (`parent.UserConstructionScript`))